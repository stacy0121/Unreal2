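; BP_PrisonBreakGameMode is the Prison Break game mode that sets up a second local player at startup.
; On BeginPlay it creates the player, destroys its default pawn, then spawns BP_PlayerB at the game mode's transform and possesses it.
; Unconnected nodes for possessing BP_PlayerA or BP_CCTV with the first controller never run.
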(event `self.ReceiveBeginPlay`
  (bind _returnvalue (`GameplayStatics.CreatePlayer` -1))
  (`self.K2_DestroyActor` (`Controller.K2_GetPawn` _returnvalue))
  (bind _returnvalue_2 (`|SpawnActorFromClass` "/Game/Blueprint/BP_PlayerB.BP_PlayerB_C" (`self.GetTransform`) "AlwaysSpawn" "OverrideRootScale" null null))
  (`Controller.Possess` _returnvalue _returnvalue_2))

(event `Key|Q`
  (params (Key :type "Key Structure")))

(fn `UserConstructionScript`)